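; Actor component that gives an owner's skeletal mesh per-bone health and physics-driven hit reactions and breakage.
; BeginPlay adds a physical animation component and seeds health for every socket name.
; HitBone applies an impulse and enables Tick, which drives the physics blend weight from a timer, then calls DamageBone.
; DamageBone maps lost health to blend weight; at zero, BreakBone leaves that bone chain fully simulated; Death is an empty stub.
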(event `self.ReceiveTick`
  (params (DeltaSeconds :type "Float (single-precision)"))
  (set `self.Time_Remaining` (- (`KismetMathLibrary.FInterpTo` (`self.Time_Remaining`) 0.0 0.0 (+ (/ (`self.Hit_Reaction_Damage`) 10.0) 0.5)) (* DeltaSeconds 0.1)))
  (if (<= (`self.Time_Remaining`) 0.0)
    (set `self.Time_Remaining` 0.0)
    (`self.SetComponentTickEnabled` false)
    (`self.Damage_Bone` (`self.Hit_Bone_Reaction`) (`self.Hit_Reaction_Damage`) (`self.Hit_Reaction_Impulse_Vel`))
    (else
      (`SkeletalMeshComponent.SetAllBodiesBelowPhysicsBlendWeight` (`self.Mesh`) (`self.Hit_Bone_Reaction`) (`KismetMathLibrary.FMin` (`self.Time_Remaining`) 1.0) false true))))

(event `self.ReceiveBeginPlay`
  (bind _returnvalue (`|AddComponentByClass` (`self.GetOwner`) "/Script/Engine.PhysicalAnimationComponent"))
  (set `self.Physical_Animation_Component` _returnvalue)
  (bind _skeletal_mesh_component (message `/Game/Skeleton_Damage_System/BPI_Implements_Skeleton_Damage.Get_Mesh` (`self.GetOwner`)))
  (bind _output_get (set `self.Mesh` _skeletal_mesh_component))
  (for _array_element (`SceneComponent.GetAllSocketNames` _output_get)
    (`BlueprintMapLibrary.Map_Add` (`self.Bones - Health`) _array_element 100.0)
    (`BlueprintMapLibrary.Map_Add` (`self.Bones - Broken`) _array_element)))

(fn `Break_Bone`
  (params (Broken_Area :type Name) (Impulse_Strength :type "Vector Structure"))
  (if (not (`BlueprintMapLibrary.Map_Find` (`self.Bones - Broken`) Broken_Area))
    (`KismetSystemLibrary.PrintString` (`KismetStringLibrary.Concat_StrStr` "BREAKING BONES IN AREA : " (`KismetStringLibrary.Conv_NameToString` Broken_Area)))
    (`BlueprintMapLibrary.Map_Add` (`self.Bones - Broken`) Broken_Area true)
    (`SkeletalMeshComponent.SetAllBodiesBelowSimulatePhysics` (`self.Mesh`) Broken_Area true true)
    (`PrimitiveComponent.AddImpulse` (`self.Mesh`) Impulse_Strength Broken_Area true)
    (bind _keys (`BlueprintMapLibrary.Map_Keys` (`self.Bones - Health`)))
    (for _array_element _keys
      (if (`SkinnedMeshComponent.BoneIsChildOf` (`self.Mesh`) _array_element Broken_Area)
        (`SkeletalMeshComponent.SetAllBodiesBelowPhysicsBlendWeight` (`self.Mesh`) _array_element 1.0 false true)
        (`BlueprintMapLibrary.Map_Add` (`self.Bones - Health`) _array_element)))))

(fn `Damage_Bone`
  (params (Bone_To_Damage :type Name) (Damage_To_Deal :type "Float (double-precision)") (Impulse_Strength :type "Vector Structure"))
  (locals (Local_Bone :type Name) (Local_Damage :type "Float (double-precision)") (Local_Impulse_Vel :type "Vector Structure"))
  (bind _value (`BlueprintMapLibrary.Map_Find` (`self.Bones - Health`) (`local.Local_Bone`)))
  (set `local.Local_Bone` Bone_To_Damage)
  (set `local.Local_Damage` Damage_To_Deal)
  (set `local.Local_Impulse_Vel` Impulse_Strength)
  (`BlueprintMapLibrary.Map_Add` (`self.Bones - Health`) (`local.Local_Bone`) (- (`BlueprintMapLibrary.Map_Find` (`self.Bones - Health`) (`local.Local_Bone`)) (`KismetMathLibrary.FClamp` (`local.Local_Damage`) 0.0 100.0)))
  (`SkeletalMeshComponent.SetAllBodiesBelowSimulatePhysics` (`self.Mesh`) (`local.Local_Bone`) true true)
  (`SkeletalMeshComponent.SetAllBodiesBelowPhysicsBlendWeight` (`self.Mesh`) (`local.Local_Bone`) (`KismetMathLibrary.FClamp` (- 1.0 (/ (`BlueprintMapLibrary.Map_Find` (`self.Bones - Health`) (`local.Local_Bone`)) 100.0))) false true)
  (bind _keys (`BlueprintMapLibrary.Map_Keys` (`self.Bones - Health`)))
  (for _array_element _keys
    (if (`SkinnedMeshComponent.BoneIsChildOf` (`self.Mesh`) _array_element (`local.Local_Bone`))
      (`SkeletalMeshComponent.SetAllBodiesBelowPhysicsBlendWeight` (`self.Mesh`) _array_element (`KismetMathLibrary.FClamp` (- 1.0 (/ (`BlueprintMapLibrary.Map_Find` (`self.Bones - Health`) _array_element) 100.0))) false true)))
  (`KismetSystemLibrary.PrintString` (`KismetStringLibrary.Conv_DoubleToString` _value))
  (if (<= _value 0.0)
    (`self.Break_Bone` (`local.Local_Bone`) (`local.Local_Impulse_Vel`))))

(fn `Death`)

(fn `Hit_Bone`
  (params (Hit_Bone :type Name) (Damage :type "Float (double-precision)") (Hit_Impulse_Strength :type "Vector Structure"))
  (bind _hit_bone_reaction (`self.Hit_Bone_Reaction`))
  (bind _mesh (`self.Mesh`))
  (set `self.Hit_Bone_Reaction` Hit_Bone)
  (set `self.Hit_Reaction_Damage` Damage)
  (`self.SetComponentTickEnabled` true)
  (set `self.Hit_Reaction_Impulse_Vel` Hit_Impulse_Strength)
  (`SkeletalMeshComponent.SetAllBodiesBelowSimulatePhysics` _mesh _hit_bone_reaction true true)
  (`PrimitiveComponent.AddImpulse` _mesh (`self.Hit_Reaction_Impulse_Vel`) _hit_bone_reaction true))